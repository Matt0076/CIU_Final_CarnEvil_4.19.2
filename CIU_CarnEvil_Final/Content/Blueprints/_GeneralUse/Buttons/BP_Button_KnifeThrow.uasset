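; Physical VR push button, labelled from ButtonText, that loads the KnifeThrow level.
; A motion controller's FingerTip overlapping the box opens a tick gate that moves the button along local Z, clamped to PressDistance.
; Full press calls the empty ButtonAction, then ResetButton; GrabSphere leaving the box also triggers the reset.
; The reset's snap-back timeline update plays the click and opens the level after a delay, so either path loads it.
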(event `self.ReceiveTick`
  (params (DeltaSeconds :type "Float (single-precision)"))
  (bind _buttonstartlocation (`self.ButtonStartLocation`))
  (bind (_buttonstartlocation_x _buttonstartlocation_y _buttonstartlocation_z) (`KismetMathLibrary.BreakVector` (`self.ButtonStartLocation`)))
  (bind _z (.z _buttonstartlocation))
  (bind (_relativelocation_x _relativelocation_y _relativelocation_z) (`KismetMathLibrary.BreakVector` (`SceneComponent.RelativeLocation` (`self.Button`))))
  ;[1 0 0] Event Tick - button Push distance
  (`/Engine/EditorBlueprintResources/StandardMacros.Gate` true :!label _label
    (:`Exit`
      (`SceneComponent.K2_SetRelativeLocation` (`self.Button`) (`KismetMathLibrary.MakeVector` (.x (+ _buttonstartlocation (`KismetMathLibrary.MakeVector` 0.0 0.0 (.z (- (`KismetMathLibrary.InverseTransformLocation` (`self.GetTransform`) (`SceneComponent.K2_GetComponentLocation` (stale `self.Box.OnComponentBeginOverlap` _output_get))) (`self.ButtonStartLocation`)))))) (.y (+ _buttonstartlocation (`KismetMathLibrary.MakeVector` 0.0 0.0 (.z (- (`KismetMathLibrary.InverseTransformLocation` (`self.GetTransform`) (`SceneComponent.K2_GetComponentLocation` (stale `self.Box.OnComponentBeginOverlap` _output_get))) (`self.ButtonStartLocation`)))))) (`KismetMathLibrary.FClamp` (.z (+ _buttonstartlocation (`KismetMathLibrary.MakeVector` 0.0 0.0 (.z (- (`KismetMathLibrary.InverseTransformLocation` (`self.GetTransform`) (`SceneComponent.K2_GetComponentLocation` (stale `self.Box.OnComponentBeginOverlap` _output_get))) (`self.ButtonStartLocation`)))))) (- _z (`self.PressDistance`)) _z)) false false)
      ;[1 1 1] Press Button if Pressed over distance then reset button
      (if (`KismetMathLibrary.NearlyEqual_FloatFloat` _relativelocation_z (- _buttonstartlocation_z (`self.PressDistance`)) 0.1)
        (`self.ButtonAction`)
        (`self.ResetButton`)))))

(event `self.Box.OnComponentBeginOverlap`
  (params (OverlappedComponent :type "PrimitiveComponent Object Reference") (OtherActor :type "Actor Object Reference") (OtherComp :type "PrimitiveComponent Object Reference") (OtherBodyIndex :type Integer) (bFromSweep :type Boolean) (SweepResult :type "HitResult Structure (by ref)"))
  ;[1 1 1] On Component Begin Overlap - Check if right hand and allow to push
  (if (not (`self.DisablePress`))
    (bind _asbp_motion_controller (cast `/Game/VirtualRealityBP/Blueprints/BP_MotionController` OtherActor))
    (bind _fingertip (`/Game/VirtualRealityBP/Blueprints/BP_MotionController.FingerTip` _asbp_motion_controller))
    (if (== _fingertip OtherComp)
      (set `self.DisablePress` true)
      (bind _output_get (set `/Game/VirtualRealityBP/Blueprints/BP_MotionController.FingerTip` _fingertip _asbp_motion_controller))
      (set `self.ButtonStartLocation` (`SceneComponent.RelativeLocation` (`self.Button`)))
      (goto _label :!via `Open`))))

(event `ResetButton`
  ;[1 1 1] On Component End Overlap - reset the button back
  (`|ExecutionSequence` :!label _label_2
    (:`then_0`
      (goto _label :!via `Close`))
    (:`then_1`
      (bind (_direction _driver) (`Timeline|SnapBackTimeLine` :!via `PlayFromStart`)
        (:`Update`
          (`SceneComponent.K2_SetRelativeLocation` (`self.Button`) (`KismetMathLibrary.MakeVector` (.x (`self.ButtonStartLocation`)) (.y (`self.ButtonStartLocation`)) (`KismetMathLibrary.Lerp` (.z (`SceneComponent.RelativeLocation` (`self.Button`))) (.z (`self.ButtonStartLocation`)) _driver)) false false)
          (`GameplayStatics.SpawnSoundAtLocation` "/Game/Audio/_GeneralUse/CE_1_ButtonClick_Adam.CE_1_ButtonClick_Adam")
          (`KismetSystemLibrary.Delay` 0.5)
          (`GameplayStatics.OpenLevel` "KnifeThrow"))
        (:`Finished`
          (set `self.DisablePress` false))))))

(event `self.Box.OnComponentEndOverlap`
  (params (OverlappedComponent :type "PrimitiveComponent Object Reference") (OtherActor :type "Actor Object Reference") (OtherComp :type "PrimitiveComponent Object Reference") (OtherBodyIndex :type Integer))
  ;[1 1 1] On Component End Overlap - reset the button back
  (bind _asbp_motion_controller (cast `/Game/VirtualRealityBP/Blueprints/BP_MotionController` OtherActor))
  (if (== (`/Game/VirtualRealityBP/Blueprints/BP_MotionController.GrabSphere` _asbp_motion_controller) OtherComp)
    (goto _label_2)))

(fn `ButtonAction`)

(fn `UserConstructionScript`
  ;[1 1 1] Set Button Text
  (`TextRenderComponent.K2_SetText` (`self.TextRender`) (`self.ButtonText`)))