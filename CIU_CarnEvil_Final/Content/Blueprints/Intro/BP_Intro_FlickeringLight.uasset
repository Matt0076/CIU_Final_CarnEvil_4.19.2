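; Intro-scene light rig actor that flickers three spotlights (left, right and back).
; After a short startup delay on BeginPlay, a Sequence starts three endless Delay loops, one per light.
; Left and right lights get random intensities several times a second, while the back light changes intensity and random color more slowly.
; Color changes for the left and right lights exist but are left unwired.
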(event `self.ReceiveBeginPlay`
  (bind _spotlight_back (`self.SpotLight_Back`))
  (`KismetSystemLibrary.Delay` 5.0)
  (`|ExecutionSequence`
    (:`then_0`
      (`LightComponent.SetIntensity` (`self.SpotLight_Left`) (`KismetMathLibrary.RandomFloatInRange` 0.0 100000.0) :!label _label)
      (`KismetSystemLibrary.Delay` 0.2)
      (goto _label))
    (:`then_1`
      (`LightComponent.SetIntensity` (`self.SpotLight_Right`) (`KismetMathLibrary.RandomFloatInRange` 0.0 100000.0) :!label _label_2)
      (`KismetSystemLibrary.Delay` 0.2)
      (goto _label_2))
    (:`then_2`
      (`LightComponent.SetIntensity` _spotlight_back (`KismetMathLibrary.RandomFloatInRange` 0.0 100000.0) :!label _label_3)
      (`LightComponent.SetLightColor` _spotlight_back (`KismetMathLibrary.Conv_VectorToLinearColor` (`KismetMathLibrary.RandomUnitVector`)) true)
      (`KismetSystemLibrary.Delay` 2.0)
      (goto _label_3))))

(fn `UserConstructionScript`)