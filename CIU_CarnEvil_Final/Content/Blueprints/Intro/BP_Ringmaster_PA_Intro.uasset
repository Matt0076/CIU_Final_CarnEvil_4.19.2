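; BP_Ringmaster_PA_Intro plays the ringmaster's intro clips, apparently public address announcements, on a timed schedule.
; BeginPlay waits through a long initial delay, then a Sequence starts three independent delays that run in parallel.
; Each delay triggers its own component from the start, so playback order is Intro1, Intro3, then Intro2, regardless of when earlier clips finish.
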(event `self.ReceiveBeginPlay`
  (`KismetSystemLibrary.Delay` 75.0)
  (`|ExecutionSequence`
    (:`then_0`
      (`KismetSystemLibrary.Delay` 3.0)
      (`AudioComponent.Play` (`self.Intro1`) 0.0))
    (:`then_1`
      (`KismetSystemLibrary.Delay` 20.0)
      (`AudioComponent.Play` (`self.Intro3`) 0.0))
    (:`then_2`
      (`KismetSystemLibrary.Delay` 100.0)
      (`AudioComponent.Play` (`self.Intro2`) 0.0))))

(fn `UserConstructionScript`)