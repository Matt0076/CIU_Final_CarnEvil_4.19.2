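; BP_Female_PA_Intro plays timed female PA audio during the intro.
; On BeginPlay, a short delay leads into a Sequence whose branches each start their own Delay, so all timers run in parallel from the same moment.
; Each branch then plays one of the components Intro1 through Intro4 from the start, with the last branch playing Intro4 a second time.
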(event `self.ReceiveBeginPlay`
  (`KismetSystemLibrary.Delay` 1.0)
  (`|ExecutionSequence`
    (:`then_0`
      (`KismetSystemLibrary.Delay` 2.0)
      (`AudioComponent.Play` (`self.Intro1`) 0.0))
    (:`then_1`
      (`KismetSystemLibrary.Delay` 8.0)
      (`AudioComponent.Play` (`self.Intro2`) 0.0))
    (:`then_2`
      (`KismetSystemLibrary.Delay` 70.0)
      (`AudioComponent.Play` (`self.Intro3`) 0.0))
    (:`then_3`
      (`KismetSystemLibrary.Delay` 93.0)
      (`AudioComponent.Play` (`self.Intro4`) 0.0))
    (:`then_4`
      (`KismetSystemLibrary.Delay` 103.0)
      (`AudioComponent.Play` (`self.Intro4`) 0.0))))

(fn `UserConstructionScript`)