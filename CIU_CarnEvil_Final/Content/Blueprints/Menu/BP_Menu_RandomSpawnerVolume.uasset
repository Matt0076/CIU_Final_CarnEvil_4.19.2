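; BP_Menu_RandomSpawnerVolume is a menu actor that repeatedly spawns random actors from ActorList inside its Volume box.
; A gate, opened on BeginPlay and closed on EndPlay, feeds Tick into a half-second Delay that paces the spawn bursts.
; Each burst spawns one randomly picked class per list entry, tiny-scaled at random box positions, with rotation derived from a random reachable navigation point.
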(event `self.ReceiveTick`
  (params (DeltaSeconds :type "Float (single-precision)"))
  (bind _actorlist (`self.ActorList`))
  (bind _returnvalue (`BoxComponent.GetScaledBoxExtent` (`self.Volume`)))
  (bind _x (.x _returnvalue))
  (bind _y (.y _returnvalue))
  (bind _z (.z _returnvalue))
  ;[1 1 1] Event Begin Play - Randomly spawn inside the Volume and random rotation - timed here also
  (`/Engine/EditorBlueprintResources/StandardMacros.Gate` true :!label _label
    (:`Exit`
      (`KismetSystemLibrary.Delay` 0.5)
      (for _ (`self.ActorList`)
        (`|SpawnActorFromClass` (`|GetArrayItem` _actorlist (`KismetMathLibrary.RandomInteger` (`KismetArrayLibrary.Array_Length` _actorlist))) (`KismetMathLibrary.MakeTransform` (+ (`KismetMathLibrary.MakeVector` (`KismetMathLibrary.RandomFloatInRange` (* _x -1.0) _x) (`KismetMathLibrary.RandomFloatInRange` (* _y -1.0) _y) (`KismetMathLibrary.RandomFloatInRange` (* _z -1.0) _z)) (`self.K2_GetActorLocation`)) (`KismetMathLibrary.Conv_VectorToRotator` (`NavigationSystem.K2_GetRandomReachablePointInRadius` _returnvalue 10.0)) (0.015 0.015 0.015)) "Undefined" "OverrideRootScale" null null)))))

(event `self.ReceiveBeginPlay`
  ;[1 1 1] Event Begin Play - Randomly spawn inside the Volume and random rotation - timed here also
  (goto _label :!via `Open`))

(event `self.ReceiveEndPlay`
  (params (EndPlayReason :type "EEndPlayReason Enum" :default "Destroyed"))
  ;[1 1 1] Event Begin Play - Randomly spawn inside the Volume and random rotation - timed here also
  (goto _label :!via `Close`))

(fn `UserConstructionScript`)