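; Menu actor that makes three spotlights (left, right and back) flicker with random intensity and colour.
; After a short delay on BeginPlay, a Sequence starts three endless Delay-driven loops, one per light.
; Left and right re-roll at short random intervals, while the back light uses a lower intensity range and a slower fixed interval.
; Colours come from random unit vectors converted to linear colours.
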(event `self.ReceiveBeginPlay`
  (bind _spotlight_left (`self.SpotLight_Left`))
  (bind _spotlight_right (`self.SpotLight_Right`))
  (bind _spotlight_back (`self.SpotLight_Back`))
  (`KismetSystemLibrary.Delay` 5.0)
  (`|ExecutionSequence`
    (:`then_0`
      ;[1 1 1] Event begin play - Randomly set the intensity and colour of the SpotLight
      (`LightComponent.SetIntensity` _spotlight_left (`KismetMathLibrary.RandomFloatInRange` 0.0 500000.0) :!label _label)
      (`LightComponent.SetLightColor` _spotlight_left (`KismetMathLibrary.Conv_VectorToLinearColor` (`KismetMathLibrary.RandomUnitVector`)) true)
      (`KismetSystemLibrary.Delay` (`KismetMathLibrary.RandomFloatInRange` 0.05 0.2))
      (goto _label))
    (:`then_1`
      ;[1 1 1] Event begin play - Randomly set the intensity and colour of the SpotLight
      (`LightComponent.SetIntensity` _spotlight_right (`KismetMathLibrary.RandomFloatInRange` 0.0 500000.0) :!label _label_2)
      (`LightComponent.SetLightColor` _spotlight_right (`KismetMathLibrary.Conv_VectorToLinearColor` (`KismetMathLibrary.RandomUnitVector`)) true)
      (`KismetSystemLibrary.Delay` (`KismetMathLibrary.RandomFloatInRange` 0.05 0.2))
      (goto _label_2))
    (:`then_2`
      ;[1 1 1] Event begin play - Randomly set the intensity and colour of the SpotLight
      (`LightComponent.SetIntensity` _spotlight_back (`KismetMathLibrary.RandomFloatInRange` 0.0 200000.0) :!label _label_3)
      (`LightComponent.SetLightColor` _spotlight_back (`KismetMathLibrary.Conv_VectorToLinearColor` (`KismetMathLibrary.RandomUnitVector`)) true)
      (`KismetSystemLibrary.Delay` 1.07)
      (goto _label_3))))

(fn `UserConstructionScript`)