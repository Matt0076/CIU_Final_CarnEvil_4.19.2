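; Bowling ball spawner that replaces a ball with a random one after it leaves the spawner's respawn box, intended for when the user picks it up.
; End overlap checks the departing actor for BP_AngryBall or BP_FearBall in parallel Sequence branches.
; After a short delay, the matching branch plays a quiet buzzer and spawns a random class from ActorList at the spawner's transform.
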(event `self.Respawn_Box.OnComponentEndOverlap`
  (params (OverlappedComponent :type "PrimitiveComponent Object Reference") (OtherActor :type "Actor Object Reference") (OtherComp :type "PrimitiveComponent Object Reference") (OtherBodyIndex :type Integer))
  (bind _actorlist (`self.ActorList`))
  (bind _actorlist_2 (`self.ActorList`))
  ;[1 1 1] Actor end Overlap - respawn a random ball once user picks it up.
  (`|ExecutionSequence`
    (:`then_0`
      (cast `/Game/Blueprints/Bowling/BP_AngryBall` OtherActor)
      (`KismetSystemLibrary.Delay` 3.0)
      (`GameplayStatics.SpawnSoundAtLocation` "/Game/Audio/_GeneralUse/CE_15_BuzzerToStartActivity_IPR_Adam.CE_15_BuzzerToStartActivity_IPR_Adam" (`self.K2_GetActorLocation`) (`self.K2_GetActorRotation`) 0.05 1.25)
      (`|SpawnActorFromClass` (`|GetArrayItem` _actorlist (`KismetMathLibrary.RandomInteger` (`KismetArrayLibrary.Array_Length` _actorlist))) (`self.GetTransform`) "Undefined" "OverrideRootScale" null null))
    (:`then_1`
      (cast `/Game/Blueprints/Bowling/BP_FearBall` OtherActor)
      (`KismetSystemLibrary.Delay` 3.0)
      (`GameplayStatics.SpawnSoundAtLocation` "/Game/Audio/_GeneralUse/CE_15_BuzzerToStartActivity_IPR_Adam.CE_15_BuzzerToStartActivity_IPR_Adam" (`self.K2_GetActorLocation`) (`self.K2_GetActorRotation`) 0.05 1.25)
      (`|SpawnActorFromClass` (`|GetArrayItem` _actorlist_2 (`KismetMathLibrary.RandomInteger` (`KismetArrayLibrary.Array_Length` _actorlist_2))) (`self.GetTransform`) "Undefined" "OverrideRootScale" null null))))

(fn `UserConstructionScript`)