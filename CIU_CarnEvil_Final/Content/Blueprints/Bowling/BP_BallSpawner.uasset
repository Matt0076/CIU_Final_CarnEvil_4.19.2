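; Bowling ball spawner that supplies balls at its root component's location and rotation, with a sound cue before each spawn.
; On BeginPlay it waits, plays a buzzer and spawns the first ball, always a BP_AngryBall.
; When any actor ends overlap with it, it waits, plays a second sound, pauses again and spawns a class picked at random from an array.
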(event `self.ReceiveBeginPlay`
  (bind _defaultsceneroot (`self.DefaultSceneRoot`))
  (bind _returnvalue (`SceneComponent.K2_GetComponentLocation` _defaultsceneroot))
  ;[1 1 1] Event Begin Play - Spawn Ball
  (`KismetSystemLibrary.Delay` 10.0)
  (`GameplayStatics.SpawnSoundAtLocation` "/Game/Audio/_GeneralUse/CE_15_BuzzerToStartActivity_IPR_Adam.CE_15_BuzzerToStartActivity_IPR_Adam" _returnvalue (struct) 0.05 1.25)
  (`|SpawnActorFromClass` "/Game/Blueprints/Bowling/BP_AngryBall.BP_AngryBall_C" (`KismetMathLibrary.MakeTransform` _returnvalue (`SceneComponent.K2_GetComponentRotation` _defaultsceneroot)) "Undefined" "OverrideRootScale" null null))

(event `self.ReceiveActorEndOverlap`
  (params (OtherActor :type "Actor Object Reference"))
  (bind _defaultsceneroot (`self.DefaultSceneRoot`))
  (bind _array (`self.Array`))
  (bind _returnvalue (`SceneComponent.K2_GetComponentLocation` _defaultsceneroot))
  ;[1 1 1] Actor end overlap - Spawn ball randomly from an array
  (`KismetSystemLibrary.Delay` 2.5)
  (`GameplayStatics.SpawnSoundAtLocation` "/Game/Audio/Bowling/BowlingBalls/Bowling_DoYouevenKnow___.Bowling_DoYouevenKnow___" _returnvalue (struct) 0.05 1.25)
  (`KismetSystemLibrary.Delay` 1.0)
  (`|SpawnActorFromClass` (`|GetArrayItem` _array (`KismetMathLibrary.RandomInteger` (`KismetArrayLibrary.Array_Length` _array))) (`KismetMathLibrary.MakeTransform` _returnvalue (`SceneComponent.K2_GetComponentRotation` _defaultsceneroot)) "Undefined" "OverrideRootScale" null null))

(fn `UserConstructionScript`)