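; Spawner for the ClownBall game that replaces an eyeball ball once it leaves the respawn trigger, such as when the player picks it up.
; When a BP_EyeBall ends overlap with the trigger, it waits briefly, plays a quiet buzzer and spawns a random class from ActorList.
; The sound and spawn both use RespawnBox's relative location as a world position, with the world-location node left unused.
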(event `self.Respawn_BoxTrigger.OnComponentEndOverlap`
  (params (OverlappedComponent :type "PrimitiveComponent Object Reference") (OtherActor :type "Actor Object Reference") (OtherComp :type "PrimitiveComponent Object Reference") (OtherBodyIndex :type Integer))
  (bind _actorlist (`self.ActorList`))
  (bind _relativelocation (`SceneComponent.RelativeLocation` (`self.RespawnBox`)))
  ;[1 1 1] Actor end Overlap - respawn a random ball once user picks it up.
  (cast `/Game/Blueprints/ClownBall/BP_EyeBall` OtherActor)
  (`KismetSystemLibrary.Delay` 1.0)
  (`GameplayStatics.SpawnSoundAtLocation` "/Game/Audio/_GeneralUse/CE_15_BuzzerToStartActivity_IPR_Adam.CE_15_BuzzerToStartActivity_IPR_Adam" _relativelocation (struct) 0.05 1.25)
  (`|SpawnActorFromClass` (`|GetArrayItem` _actorlist (`KismetMathLibrary.RandomInteger` (`KismetArrayLibrary.Array_Length` _actorlist))) (`KismetMathLibrary.Conv_VectorToTransform` _relativelocation) "Undefined" "OverrideRootScale" null null))

(fn `UserConstructionScript`)