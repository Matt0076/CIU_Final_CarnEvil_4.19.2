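; BP_HeartBallSpawner is a timed launcher that spawns short-lived BP_Heart actors at its RespawnBox.
; Tick drives a chain of latent Delays, with FireInterval pacing the shots instead of a timer.
; Each shot plays an emitter and warning buzzer, then after a brief pause a firing sound and a scaled-down heart spawn, with a final Delay leading to that heart's destruction.
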(event `self.ReceiveTick`
  (params (DeltaSeconds :type "Float (single-precision)"))
  (bind _respawnbox (`self.RespawnBox`))
  (bind _returnvalue (`SceneComponent.K2_GetComponentRotation` _respawnbox))
  (bind _returnvalue_2 (`SceneComponent.K2_GetComponentLocation` _respawnbox))
  ;[1 1 1] Fire - Spawn Heart From Target Point - Timed
  (`KismetSystemLibrary.Delay` 1.0)
  (`KismetSystemLibrary.Delay` (`self.FireInterval`))
  (`GameplayStatics.SpawnEmitterAtLocation` null _returnvalue_2 _returnvalue)
  (`GameplayStatics.PlaySoundAtLocation` "/Game/Audio/_GeneralUse/CE_15_BuzzerToStartActivity_IPR_Adam.CE_15_BuzzerToStartActivity_IPR_Adam" _returnvalue_2 (struct) 0.05 1.5)
  (`KismetSystemLibrary.Delay` 0.5)
  (`GameplayStatics.PlaySoundAtLocation` "/Game/Audio/HeartBall/CE_16_HeartBeingFired_IPR_Adam.CE_16_HeartBeingFired_IPR_Adam" _returnvalue_2 (struct) 0.1 0.65)
  (bind _returnvalue_3 (`|SpawnActorFromClass` "/Game/Blueprints/HeartBall/BP_Heart.BP_Heart_C" (`KismetMathLibrary.MakeTransform` _returnvalue_2 _returnvalue (0.1 0.1 0.1)) "Undefined" "OverrideRootScale" null null))
  (`KismetSystemLibrary.Delay` 7.5)
  (`self.K2_DestroyActor` _returnvalue_3))

(fn `UserConstructionScript`)