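; BP_HeartBall_10PointsTrigger is a 10-point scoring trigger in the HeartBall game.
; When its box is overlapped, it sends a HandleUpdateScore message with a value to the overlapping actor.
; Its own HandleUpdateScore event adds the received value to PlayerScore10Points and calls UpdateScoreDisplay.
; That display function is empty, as its nodes for writing to BP_HeartBall_TotalScoreDisplay are disconnected, and debug prints trace each step.
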(event `EventHandleUpdateScore`
  (params (Value :type Integer :default 10))
  (`self.UpdateScore` Value)
  (`KismetSystemLibrary.PrintString` "HANDLE UPDATE SCORE  TRIGGERED"))

(event `self.TriggerBox_10Points.OnComponentBeginOverlap`
  (params (OverlappedComponent :type "PrimitiveComponent Object Reference") (OtherActor :type "Actor Object Reference") (OtherComp :type "PrimitiveComponent Object Reference") (OtherBodyIndex :type Integer) (bFromSweep :type Boolean) (SweepResult :type "HitResult Structure (by ref)"))
  (message `/Game/Blueprints/_GeneralUse/BPI_ScoreController.HandleUpdateScore` OtherActor (stale `EventHandleUpdateScore` Value))
  (`KismetSystemLibrary.PrintString` "10 POINTS TRIGGERED"))

(fn `UpdateScore`
  (params (ScoreToAdd :type Integer :default 0))
  (bind _output_get (set `self.PlayerScore10Points` (+ ScoreToAdd (`self.PlayerScore10Points`))))
  (`self.UpdateScoreDisplay` _output_get)
  (`KismetSystemLibrary.PrintString` "UPDATE SCORE DISPLAY TRIGGERED"))

(fn `UpdateScoreDisplay`
  (params (Score :type Integer)))

(fn `UserConstructionScript`)