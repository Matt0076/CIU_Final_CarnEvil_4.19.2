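; BP_HeartSpawner is an actor that periodically fires BP_Heart actors into the level.
; Tick drives a chain of latent Delays: a fixed wait, then FireInterval, then a firing sound and a short pause before the spawn.
; Each heart spawns at one-tenth scale using the Box component's world location and rotation.
; The firing sound plays at the world origin rather than at the spawner.
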(event `self.ReceiveTick`
  (params (DeltaSeconds :type "Float (single-precision)"))
  (bind _box (`self.Box`))
  (`KismetSystemLibrary.Delay` 5.0)
  (`KismetSystemLibrary.Delay` (`KismetMathLibrary.Conv_IntToDouble` (`self.FireInterval`)))
  (`GameplayStatics.SpawnSoundAtLocation` "/Game/Audio/HeartBall/CE_16_HeartBeingFired_IPR_Adam.CE_16_HeartBeingFired_IPR_Adam")
  (`KismetSystemLibrary.Delay` 0.5)
  (`|SpawnActorFromClass` "/Game/Blueprints/HeartBall/BP_Heart.BP_Heart_C" (`KismetMathLibrary.MakeTransform` (`SceneComponent.K2_GetComponentLocation` _box) (`SceneComponent.K2_GetComponentRotation` _box) (0.1 0.1 0.1)) "Undefined" "OverrideRootScale" null null))

(fn `UserConstructionScript`)