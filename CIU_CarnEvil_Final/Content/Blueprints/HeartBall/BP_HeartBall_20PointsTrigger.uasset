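; BP_HeartBall_20PointsTrigger is a scoring trigger for the HeartBall game that reacts to BP_Heart actors entering its box.
; Despite its name, overlap adds 10 to its own PlayerScore and writes that value onto the first BP_HeartBall_TotalScoreDisplay found, plus a debug print.
; A separate HandleUpdateScore event passes 20 points to the display's UpdateScoreDisplay, using the display reference cached on overlap.
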(event `/Game/Blueprints/_GeneralUse/BPI_ScoreController.HandleUpdateScore`
  (params (`10` :type Integer) (`20` :type Integer) (`40` :type Integer))
  (`self.UpdateScore` `20`))

(event `self.TriggerBox_10Points.OnComponentBeginOverlap`
  (params (OverlappedComponent :type "PrimitiveComponent Object Reference") (OtherActor :type "Actor Object Reference") (OtherComp :type "PrimitiveComponent Object Reference") (OtherBodyIndex :type Integer) (bFromSweep :type Boolean) (SweepResult :type "HitResult Structure (by ref)"))
  (cast `/Game/Blueprints/HeartBall/BP_Heart` OtherActor)
  (bind _outactors (`GameplayStatics.GetAllActorsOfClass` "/Game/Blueprints/HeartBall/BP_HeartBall_TotalScoreDisplay.BP_HeartBall_TotalScoreDisplay_C"))
  (bind _output_get (set `self.HeartBall Total Display Score` (`|GetArrayItem` _outactors)))
  (bind _output_get_2 (set `self.PlayerScore` (+ (`self.PlayerScore`) 10)))
  (`TextRenderComponent.K2_SetText` (`/Game/Blueprints/HeartBall/BP_HeartBall_TotalScoreDisplay.TextRender_TotalScoreDisplay` _output_get) (`KismetTextLibrary.Conv_IntToText` _output_get_2))
  (`KismetSystemLibrary.PrintString` "Hello"))

(fn `UpdateScore`
  (params (`Score to Add` :type Integer))
  (`/Game/Blueprints/HeartBall/BP_HeartBall_TotalScoreDisplay.UpdateScoreDisplay` (`self.HeartBall Total Display Score`) 0 `Score to Add` 0))

(fn `UserConstructionScript`)