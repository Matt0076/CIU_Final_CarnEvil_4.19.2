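; BP_HeartBall_TotalScoreDisplay is the text-render score display for the HeartBall game.
; Three update events each fetch the first 10, 20 or 40-point trigger actor, the first two after a short delay, then share one display call.
; That call reads PlayerScore from all three cached triggers and adds fixed offsets.
; UpdateScoreDisplay renders only the 10-point value, ignoring the other two, so no total is summed.
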(event `UpdateScoreWhenTriggered1`
  (`KismetSystemLibrary.Delay` 0.2)
  (bind _outactors (`GameplayStatics.GetAllActorsOfClass` "/Game/Blueprints/HeartBall/BP_HeartBall_10PointsTrigger.BP_HeartBall_10PointsTrigger_C"))
  (bind _asbp_heart_ball_10points_trigger (cast `/Game/Blueprints/HeartBall/BP_HeartBall_10PointsTrigger` (`|GetArrayItem` _outactors)))
  (`self.UpdateScoreDisplay` (+ (`/Game/Blueprints/HeartBall/BP_HeartBall_10PointsTrigger.PlayerScore` _asbp_heart_ball_10points_trigger) 10) (+ (`/Game/Blueprints/HeartBall/BP_HeartBall_20PointsTrigger.PlayerScore` (stale `UpdateScoreWhenTriggered2` _asbp_heart_ball_20points_trigger)) 10) (+ (`/Game/Blueprints/HeartBall/BP_HeartBall_40PointsTrigger.PlayerScore` (stale `UpdateScoreWhenTriggered3` _asbp_heart_ball_40points_trigger)) 20) :!label _label))

(event `UpdateScoreWhenTriggered2`
  (`KismetSystemLibrary.Delay` 0.2)
  (bind _outactors (`GameplayStatics.GetAllActorsOfClass` "/Game/Blueprints/HeartBall/BP_HeartBall_20PointsTrigger.BP_HeartBall_20PointsTrigger_C"))
  (bind _asbp_heart_ball_20points_trigger (cast `/Game/Blueprints/HeartBall/BP_HeartBall_20PointsTrigger` (`|GetArrayItem` _outactors)))
  (goto _label))

(event `UpdateScoreWhenTriggered3`
  (bind _outactors (`GameplayStatics.GetAllActorsOfClass` "/Game/Blueprints/HeartBall/BP_HeartBall_40PointsTrigger.BP_HeartBall_40PointsTrigger_C"))
  (bind _asbp_heart_ball_40points_trigger (cast `/Game/Blueprints/HeartBall/BP_HeartBall_40PointsTrigger` (`|GetArrayItem` _outactors)))
  (goto _label))

(fn `UpdateScoreDisplay`
  (params (Score10 :type Integer) (Score20 :type Integer) (Score40 :type Integer))
  (`TextRenderComponent.K2_SetText` (`self.TextRender_TotalScoreDisplay`) (`KismetTextLibrary.Conv_IntToText` Score10 false true 2)))

(fn `UserConstructionScript`)