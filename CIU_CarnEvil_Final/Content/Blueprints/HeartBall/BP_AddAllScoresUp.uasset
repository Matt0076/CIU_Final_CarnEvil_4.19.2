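; BP_AddAllScoresUp totals HeartBall scores from the 10, 20 and 40-point triggers for the total score display.
; AddScoresUp adds fixed offsets to each first trigger's PlayerScore, then sets the display text.
; UpdateScoreDisplay and the return value receive the sum cast through bool, losing its magnitude.
; All Sequence branches share one update-and-return path, so the first returns before the 20 and 40-point lookups run.
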(fn `AddScoresUp`
  (returns (TotalOfAllScore :type Boolean))
  (`|ExecutionSequence`
    (:`then_0`
      (bind _outactors (`GameplayStatics.GetAllActorsOfClass` "/Game/Blueprints/HeartBall/BP_HeartBall_10PointsTrigger.BP_HeartBall_10PointsTrigger_C")))
    (:`then_1`
      (bind _outactors_2 (`GameplayStatics.GetAllActorsOfClass` "/Game/Blueprints/HeartBall/BP_HeartBall_20PointsTrigger.BP_HeartBall_20PointsTrigger_C")))
    (:`then_2`
      (bind _outactors_3 (`GameplayStatics.GetAllActorsOfClass` "/Game/Blueprints/HeartBall/BP_HeartBall_40PointsTrigger.BP_HeartBall_40PointsTrigger_C"))))
  (bind _outactors_4 (`GameplayStatics.GetAllActorsOfClass` "/Game/Blueprints/HeartBall/BP_HeartBall_TotalScoreDisplay.BP_HeartBall_TotalScoreDisplay_C"))
  (bind _output_get (set `self.BP_HeartballTotalDisplayScore` (`|GetArrayItem` _outactors_4)))
  (bind _returnvalue (+ (+ (`/Game/Blueprints/HeartBall/BP_HeartBall_10PointsTrigger.PlayerScore` (`|GetArrayItem` _outactors)) 5) (+ (`/Game/Blueprints/HeartBall/BP_HeartBall_20PointsTrigger.PlayerScore` (`|GetArrayItem` _outactors_2)) 10) (+ (`/Game/Blueprints/HeartBall/BP_HeartBall_40PointsTrigger.PlayerScore` (`|GetArrayItem` _outactors_3)) 20)))
  (bind _returnvalue_2 (`KismetMathLibrary.Conv_IntToBool` _returnvalue))
  (bind _returnvalue_3 (`KismetMathLibrary.Conv_BoolToInt` _returnvalue_2))
  (`/Game/Blueprints/HeartBall/BP_HeartBall_TotalScoreDisplay.UpdateScoreDisplay` _output_get _returnvalue_3 _returnvalue_3 _returnvalue_3)
  (`TextRenderComponent.K2_SetText` (`/Game/Blueprints/HeartBall/BP_HeartBall_TotalScoreDisplay.TextRender_TotalScoreDisplay` _output_get) (`KismetTextLibrary.Conv_IntToText` _returnvalue))
  (return _returnvalue_2))