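; BP_Knife is a throwable knife that the motion controller can pick up and drop, meant to stick into a target backboard.
; Pickup disables mesh physics and attaches the knife to the given component, while Drop re-enables physics and detaches it.
; On hit, a surface-type switch with only a default branch re-enables physics, attaches the mesh to the hit component and plays a CompileFailed sound at world origin.
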(event `/Game/VirtualRealityBP/Blueprints/PickupActorInterface.Pickup`
  (params (AttachTo :type "SceneComponent Object Reference"))
  ;[1 1 1] Pick up and drop object
  (`PrimitiveComponent.SetSimulatePhysics` (`self.StaticMeshComponent`) false)
  (`SceneComponent.K2_AttachToComponent` (`self.K2_GetRootComponent`) AttachTo "None" "KeepWorld" "KeepWorld" "KeepWorld" false))

(event `/Game/VirtualRealityBP/Blueprints/PickupActorInterface.Drop`
  ;[1 1 1] Pick up and drop object
  (`PrimitiveComponent.SetSimulatePhysics` (`self.StaticMeshComponent`) true)
  (`self.K2_DetachFromActor` "KeepWorld" "KeepWorld" "KeepWorld"))

(event `self.StaticMeshComponent.OnComponentHit`
  (params (HitComponent :type "PrimitiveComponent Object Reference") (OtherActor :type "Actor Object Reference") (OtherComp :type "PrimitiveComponent Object Reference") (NormalImpulse :type "Vector Structure") (Hit :type "HitResult Structure (by ref)"))
  (bind (_bblockinghit _binitialoverlap _time _distance _location _impactpoint _normal _impactnormal _physmat _hitactor _hitcomponent) (`GameplayStatics.BreakHitResult` Hit))
  ;[1 1 1] On Component Hit - Knife Sticks to Target Backboard (Use sticky Physics material in override for any other objects for the knife to stick to)
  (switch `EPhysicalSurface` (`PhysicalMaterial.SurfaceType` _physmat)
    (:`SurfaceType_Default`
      (`PrimitiveComponent.SetSimulatePhysics` (`self.StaticMeshComponent`) true)
      (`SceneComponent.K2_AttachToComponent` (`self.StaticMeshComponent`) _hitcomponent "None" "KeepWorld" "KeepWorld" "KeepWorld" true)
      (`GameplayStatics.SpawnSoundAtLocation` "/Engine/EditorSounds/Notifications/CompileFailed.CompileFailed"))))

(fn `UserConstructionScript`)